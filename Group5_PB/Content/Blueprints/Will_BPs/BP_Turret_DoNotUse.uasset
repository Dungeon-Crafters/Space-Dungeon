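; Turret actor, named as not for use, that tracks and fires at a BP_Player inside its range.
; TurretRange overlap stores the player and opens a Tick gate, which closes when a player leaves.
; While open, the Head interpolates toward the player's mesh using a fixed delta time of 1.0, so turning is frame-rate dependent.
; SpawnProjectile spawns an actor at the ProjectileSpawn transform, throttled by FireDelay against game time.
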(event `self.ReceiveTick`
  (params (DeltaSeconds :type "Float (single-precision)"))
  (bind _head (`self.Head`))
  (`/Engine/EditorBlueprintResources/StandardMacros.Gate` true :!label _label
    (:`Exit`
      (`SceneComponent.K2_SetWorldRotation` (`self.Head`) (`KismetMathLibrary.RInterpTo` (`SceneComponent.K2_GetComponentRotation` _head) (`KismetMathLibrary.FindLookAtRotation` (`SceneComponent.K2_GetComponentLocation` _head) (`SceneComponent.K2_GetComponentLocation` (`Character.Mesh` (stale `self.Turret Range.OnComponentBeginOverlap` _asbp_player)))) 1.0 (`self.Turrent Rotation Speed`)) false false)
      (`self.Spawn Projectile`))))

(event `self.Turret Range.OnComponentBeginOverlap`
  (params (OverlappedComponent :type "PrimitiveComponent Object Reference") (OtherActor :type "Actor Object Reference") (OtherComp :type "PrimitiveComponent Object Reference") (OtherBodyIndex :type Integer) (bFromSweep :type Boolean) (SweepResult :type "HitResult Structure (by ref)"))
  (bind _asbp_player (cast `/Game/Blueprints/ConnorBPs/Player/BP_Player` OtherActor))
  (goto _label :!via `Open`))

(event `self.Turret Range.OnComponentEndOverlap`
  (params (OverlappedComponent :type "PrimitiveComponent Object Reference") (OtherActor :type "Actor Object Reference") (OtherComp :type "PrimitiveComponent Object Reference") (OtherBodyIndex :type Integer))
  (cast `/Game/Blueprints/ConnorBPs/Player/BP_Player` OtherActor)
  (goto _label :!via `Close`))

(fn `Spawn Projectile`
  (bind _returnvalue (`KismetSystemLibrary.GetGameTimeInSeconds`))
  (if (> _returnvalue (`self.GameTimeFire`))
    (set `self.GameTimeFire` (+ _returnvalue (`self.FireDelay`)))
    (`|SpawnActorFromClass` "/Game/Blueprints/ConnorBPs/Projectiles/BP_Bullet.BP_Bullet_C" (`SceneComponent.K2_GetComponentToWorld` (`self.Projectile Spawn`)) "Undefined" "OverrideRootScale" null null)))

(fn `UserConstructionScript`)