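; BP_Switch is a one-shot switch that animates an Activator cube when BP_Player steps on it and adds to the player's door-switch total.
; OnSwitch overlap plays the ActivatorMove timeline, lerping the spinning cube to an end marker, then resets its rotation and destroys the actor after a short delay.
; A separate SwitchCounter overlap increments DoorSwitchTotalAmount, prints it, then destroys that trigger component.
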(event `self.ReceiveBeginPlay`
  ;[1 1 1] Gets and sets the location of the small cube when the switch is activated
  (set `self.Start Location` (`SceneComponent.K2_GetComponentLocation` (`self.Activator`)))
  (set `self.End Location` (`SceneComponent.K2_GetComponentLocation` (`self.Activator End Location`)))
  (`TimelineComponent.SetPlayRate` (`self.Activator Move`) (`self.Playrate`)))

(event `self.On Switch.OnComponentBeginOverlap`
  (params (OverlappedComponent :type "PrimitiveComponent Object Reference") (OtherActor :type "Actor Object Reference") (OtherComp :type "PrimitiveComponent Object Reference") (OtherBodyIndex :type Integer) (bFromSweep :type Boolean) (SweepResult :type "HitResult Structure (by ref)"))
  (bind _rotation_speed (`self.Rotation Speed`))
  ;[1 1 1] Begins and reverses the animation of the cube (activator)
  (cast `/Game/Blueprints/ConnorBPs/Player/BP_Player` OtherActor)
  (bind (_direction _newtrack_0) (`Timeline|Activator Move`)
    (:`Update`
      ;[1 1 1] Adds the rotation behavior and controls rotating speed
      (`SceneComponent.K2_AddRelativeRotation` (`self.Activator`) (`KismetMathLibrary.MakeRotator` _rotation_speed 0.0 _rotation_speed) false false)
      ;[1 1 1] Sets up the start and ending locations for the animation
      (`SceneComponent.K2_SetWorldLocation` (`self.Activator`) (`KismetMathLibrary.VLerp` (`self.Start Location`) (`self.End Location`) _newtrack_0) false false))
    (:`Finished`
      ;[1 1 1] Resets the rotation of the Activator cube so it ends evenly
      (`SceneComponent.K2_SetRelativeRotation` :`self` (`self.Activator`))
      ;[1 1 1] Remove switch after X seconds
      (`KismetSystemLibrary.Delay` 1.0)
      (`self.K2_DestroyActor`))))

(event `self.On Switch.OnComponentEndOverlap`
  (params (OverlappedComponent :type "PrimitiveComponent Object Reference") (OtherActor :type "Actor Object Reference") (OtherComp :type "PrimitiveComponent Object Reference") (OtherBodyIndex :type Integer))
  ;[1 1 1] Begins and reverses the animation of the cube (activator)
  (cast `/Game/Blueprints/ConnorBPs/Player/BP_Player` OtherActor))

(event `self.Switch Counter.OnComponentBeginOverlap`
  (params (OverlappedComponent :type "PrimitiveComponent Object Reference") (OtherActor :type "Actor Object Reference") (OtherComp :type "PrimitiveComponent Object Reference") (OtherBodyIndex :type Integer) (bFromSweep :type Boolean) (SweepResult :type "HitResult Structure (by ref)"))
  (bind _asbp_player (cast `/Game/Blueprints/ConnorBPs/Player/BP_Player` OtherActor))
  (bind _output_get (set `/Game/Blueprints/ConnorBPs/Player/BP_Player.DoorSwitch_TotalAmount` (+ (`/Game/Blueprints/ConnorBPs/Player/BP_Player.DoorSwitch_TotalAmount` _asbp_player) (`self.SwitchCounter`)) _asbp_player))
  (`KismetSystemLibrary.PrintString` (`KismetStringLibrary.Conv_IntToString` _output_get))
  (`ActorComponent.K2_DestroyComponent` (`self.Switch Counter`)))

(fn `UserConstructionScript`)