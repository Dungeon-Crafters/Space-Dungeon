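; BP_StaticToGrenadeCube is a stand-in box that becomes a destructible box when a grenade reaches it.
; When a Grenade overlaps GrenadeDetector, it destroys itself, spawns BP_GrenadeBox with the same location and rotation for a seamless swap, then calls Death on it.
; An unconnected alternative branch instead enables physics and applies delayed radius damage to the spawned destructible.
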(event `self.Grenade Detector.OnComponentBeginOverlap`
  (params (OverlappedComponent :type "PrimitiveComponent Object Reference") (OtherActor :type "Actor Object Reference") (OtherComp :type "PrimitiveComponent Object Reference") (OtherBodyIndex :type Integer) (bFromSweep :type Boolean) (SweepResult :type "HitResult Structure (by ref)"))
  ;[1 1 1] Turns static mesh into the destructible box.  Will copy the location and rotation of the boxes it is replacing so the change is seamless.
  (cast `/Game/Blueprints/Colin_BPs/Grenade` OtherActor)
  (`self.K2_DestroyActor`)
  (bind _returnvalue (`|SpawnActorFromClass` "/Game/Blueprints/Will_BPs/BP_GrenadeBox.BP_GrenadeBox_C" (`KismetMathLibrary.MakeTransform` (`self.K2_GetActorLocation`) (`self.K2_GetActorRotation`)) "Undefined" "OverrideRootScale" null null))
  (`/Game/Blueprints/Will_BPs/BP_GrenadeBox.Death` _returnvalue))

(fn `UserConstructionScript`)