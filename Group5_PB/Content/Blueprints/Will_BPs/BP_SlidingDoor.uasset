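; BP_SlidingDoor is a door that slides open when something enters its trigger, provided enough switches have been collected.
; On overlap, it compares the game instance's switch total against a required amount, printing a message on screen if short.
; Otherwise, a timeline, with its play rate set at BeginPlay, lerps the door from its starting world location to a destination component's location.
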(event `self.ReceiveBeginPlay`
  ;[1 1 1] Gets the start and sets the end location of the door.
  (set `self.Start Location` (`SceneComponent.K2_GetComponentLocation` (`self.Door`)))
  (set `self.End Location` (`SceneComponent.K2_GetComponentLocation` (`self.Door Destination`)))
  (`TimelineComponent.SetPlayRate` (`self.Platform Timeline`) (`self.Playrate`)))

(event `self.Door Collider.OnComponentBeginOverlap`
  (params (OverlappedComponent :type "PrimitiveComponent Object Reference") (OtherActor :type "Actor Object Reference") (OtherComp :type "PrimitiveComponent Object Reference") (OtherBodyIndex :type Integer) (bFromSweep :type Boolean) (SweepResult :type "HitResult Structure (by ref)"))
  ;[1 1 1] Checks to see if player has the required amount of switches.  If so, opens the door.  If not, prints out a message.
  (bind _asbp_gi (cast `/Game/Blueprints/Will_BPs/BP_GI` (`GameplayStatics.GetGameInstance`)))
  (if (>= (`/Game/Blueprints/Will_BPs/BP_GI.TotalAmountOfSwitches` _asbp_gi) (`self.RequiredSwitchAmounts`))
    (cast `ActorComponent` (`self.Door`))
    (bind (_direction _newtrack_0) (`Timeline|Platform Timeline`)
      (:`Update`
        (`SceneComponent.K2_SetWorldLocation` (`self.Door`) (`KismetMathLibrary.VLerp` (`self.Start Location`) (`self.End Location`) _newtrack_0) false false)))
    (else
      (`KismetSystemLibrary.PrintString` (`self.Print String Message`) true true (struct :`R` 1.0 :`G` 0.047866 :`A` 1.0)))))

(fn `UserConstructionScript`)