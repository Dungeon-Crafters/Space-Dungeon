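; BP_EnemyTurret is a stationary enemy turret that turns toward a seen player and fires projectiles at them.
; PawnSensing drives a one-time alert beep, actor rotation with the base's rotation reset, and delayed BP_TurretBullet shots gated by a cooldown flag.
; Its hurt box takes damage from player bullets and explosions with a material flicker, and damages players lacking invincibility frames.
; Tick destroys the turret once Health runs out.
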(event `self.PawnSensing.OnSeePawn`
  (params (Pawn :type "Pawn Object Reference"))
  (if (`self.soundOn`)
    (`GameplayStatics.PlaySoundAtLocation` "/Game/Assets/426888__thisusernameis__beep4.426888__thisusernameis__beep4" (0.0 0.0 0.0) (struct) 1.0 1.0 0.0 null null null)
    (set `self.soundOn` false))
  (bind _asbp_player (cast `/Game/Blueprints/ConnorBPs/Player/BP_Player` Pawn))
  ;[1 1 1] Allows us to set rotation and fire at the same time
  (`|ExecutionSequence`
    (:`then_0`
      ;[1 1 1] Stops the turret body from moving
      (`SceneComponent.K2_SetWorldRotation` :`self` (`self.Base`))
      ;[1 1 1] Set turret rotation
      (`self.K2_SetActorRotation` (`KismetMathLibrary.FindLookAtRotation` (`self.K2_GetActorLocation`) (`self.K2_GetActorLocation` _asbp_player))))
    (:`then_1`
      ;[1 1 1] Controls Fire behavior
      (if (`self.SpawnProjectile`)
        (`KismetSystemLibrary.Delay` 1.0)
        (`|SpawnActorFromClass` "/Game/Blueprints/Will_BPs/BP_TurretBullet.BP_TurretBullet_C" (`SceneComponent.K2_GetComponentToWorld` (`self.Projectile Spawn Location`)) "Undefined" "OverrideRootScale" null null)
        (`GameplayStatics.SpawnSoundAtLocation` "/Game/Assets/459609__bolkmar__fx-laser-shoot-b.459609__bolkmar__fx-laser-shoot-b" (0.0 0.0 0.0) (struct) 1.0 1.0 0.0 null null)
        (set `self.SpawnProjectile` false)
        (`KismetSystemLibrary.Delay` (`self.Shooting Delay`))
        (set `self.SpawnProjectile` true)))))

(event `self.ReceiveTick`
  (params (DeltaSeconds :type "Float (single-precision)"))
  ;[1 1 1] activate chase on spawn and destroy actor when health is 0
  (if (<= (`self.health`) 0)
    (`self.K2_DestroyActor`)))

(event `flicker`
  (bind _base (`self.Base`))
  ;[1 1 1] Flicker
  (`PrimitiveComponent.SetMaterial` _base 0 "/Game/Blueprints/ConnorBPs/isOff.isOff")
  (`KismetSystemLibrary.Delay` 0.1)
  (`PrimitiveComponent.SetMaterial` _base 0 "/Game/Assets/Materials/Blue.Blue"))

(event `self.EnemyHurtBox.OnComponentBeginOverlap`
  (params (OverlappedComponent :type "PrimitiveComponent Object Reference") (OtherActor :type "Actor Object Reference") (OtherComp :type "PrimitiveComponent Object Reference") (OtherBodyIndex :type Integer) (bFromSweep :type Boolean) (SweepResult :type "HitResult Structure (by ref)"))
  ;[1 1 1] Hit Player and Hit Bullet
  (`|ExecutionSequence`
    (:`then_0`
      (cast `/Game/Blueprints/ConnorBPs/Projectiles/BP_Bullet` OtherActor)
      (`|ExecutionSequence`
        (:`then_0`
          (`/Engine/EditorBlueprintResources/StandardMacros.DecrementInt` (`self.health`)))
        (:`then_1`
          (`self.flicker`))))
    (:`then_1`
      (bind _asbp_player (cast `/Game/Blueprints/ConnorBPs/Player/BP_Player` OtherActor))
      (if (not (`/Game/Blueprints/ConnorBPs/Player/BP_Player.IFrame` _asbp_player))
        (set `/Game/Blueprints/ConnorBPs/Player/BP_Player.Player Health` (- (`/Game/Blueprints/ConnorBPs/Player/BP_Player.Player Health` _asbp_player) 0.1) _asbp_player)
        (`KismetSystemLibrary.PrintString` "Ouch!")
        (set `/Game/Blueprints/ConnorBPs/Player/BP_Player.IFrame` true _asbp_player)))
    (:`then_2`
      (cast `/Game/Blueprints/Colin_BPs/Explosion` OtherActor)
      (`|ExecutionSequence`
        (:`then_0`
          (for _ (range 5)
            (`/Engine/EditorBlueprintResources/StandardMacros.DecrementInt` (`self.health`))))
        (:`then_1`
          (`self.flicker`))))))

(fn `UserConstructionScript`)