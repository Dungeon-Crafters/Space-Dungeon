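; MyProjectile is an enemy bullet that damages the player on contact.
; When its Bullet component overlaps a BP_Player without IFrame set, it subtracts a fixed amount of PlayerHealth, prints a debug message, destroys itself and sets IFrame on the player.
; Overlaps during the player's IFrame are ignored, and the bullet destroys itself after a short delay from spawn.
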(event `self.ReceiveBeginPlay`
  ;[1 1 1] Will destroy bullet after two seconds if miss player
  (`KismetSystemLibrary.Delay` 2.0)
  (`self.K2_DestroyActor`))

(event `self.Bullet.OnComponentBeginOverlap`
  (params (OverlappedComponent :type "PrimitiveComponent Object Reference") (OtherActor :type "Actor Object Reference") (OtherComp :type "PrimitiveComponent Object Reference") (OtherBodyIndex :type Integer) (bFromSweep :type Boolean) (SweepResult :type "HitResult Structure (by ref)"))
  (bind _asbp_player (cast `/Game/Blueprints/ConnorBPs/Player/BP_Player` OtherActor))
  (if (not (`/Game/Blueprints/ConnorBPs/Player/BP_Player.IFrame` _asbp_player))
    (set `/Game/Blueprints/ConnorBPs/Player/BP_Player.Player Health` (- (`/Game/Blueprints/ConnorBPs/Player/BP_Player.Player Health` _asbp_player) 0.1) _asbp_player)
    (`KismetSystemLibrary.PrintString` "Ouch!" true true (struct :`G` 0.66 :`B` 1.0 :`A` 1.0) 0.5)
    (`self.K2_DestroyActor`)
    (set `/Game/Blueprints/ConnorBPs/Player/BP_Player.IFrame` true _asbp_player)))

(fn `UserConstructionScript`)