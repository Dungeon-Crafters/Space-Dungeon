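; ThePod is a puzzle tile actor that changes material on overlap and locks once the puzzle is solved.
; Box overlap clears ActiveState on both branches, so the tile always turns Blue unless disabled.
; Update1 counts every TriggerBox regardless of state; matching the required count disables all pods and applies the Complete material.
; Adjacent-tile toggle logic is present but unconnected.
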(event `self.ReceiveTick`
  (params (DeltaSeconds :type "Float (single-precision)")))

(event `self.Box.OnComponentBeginOverlap`
  (params (OverlappedComponent :type "PrimitiveComponent Object Reference") (OtherActor :type "Actor Object Reference") (OtherComp :type "PrimitiveComponent Object Reference") (OtherBodyIndex :type Integer) (bFromSweep :type Boolean) (SweepResult :type "HitResult Structure (by ref)"))
  (bind _activestate (`self.ActiveState`))
  (bind _tilebase (`self.TileBase`))
  (if (not (`self.PuzzleDisabled`))
    (if _activestate
      (set `self.ActiveState` false)
      (else
        (set `self.ActiveState` false)))
    (if _activestate
      (`PrimitiveComponent.SetMaterial` _tilebase 0 "/Game/Assets/Materials/Orange.Orange")
      (else
        (`PrimitiveComponent.SetMaterial` _tilebase 0 "/Game/Assets/Materials/Blue.Blue")))))

(event `Update 1`
  (if (not (`self.Puzzle Solved`))
    (set `self.Active Buttons in Puzzles` 0)
    (bind _outactors (`GameplayStatics.GetAllActorsOfClass` "/Script/Engine.TriggerBox"))
    (for _ _outactors
      (if true
        (set `self.Active Buttons in Puzzles` (+ (`self.Active Buttons in Puzzles`) 1))))
    (`/Engine/EditorBlueprintResources/StandardMacros.CompareInt` (`self.Active Buttons in Puzzles`) (`self.Number Of Buttons in Puzzle`)
      (:`==`
        (if (not (`self.Puzzle01 is Solved`))
          (`|ExecutionSequence`
            (:`then_0`
              (set `self.Puzzle01 is Solved` true)
              (`|ExecutionSequence`
                (:`then_0`
                  (bind _outactors_2 (`GameplayStatics.GetAllActorsOfClass` "ThePod_C"))
                  (for _array_element _outactors_2
                    (`|ExecutionSequence`
                      (:`then_0`
                        (bind _asthe_pod (cast `/Game/Blueprints/Ivana_BP/ThePod` _array_element))
                        (set `/Game/Blueprints/Ivana_BP/ThePod.PuzzleDisabled` true _asthe_pod))
                      (:`then_1`
                        (`PrimitiveComponent.SetMaterial` (`/Game/Blueprints/Ivana_BP/ThePod.TileBase` _array_element) 0 "/Game/Blueprints/ConnorBPs/Complete.Complete")))))))))))))

(fn `UserConstructionScript`)