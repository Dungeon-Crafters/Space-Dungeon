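; AIShooterChar is an enemy AI character that roams, patrols or chases the player and fires projectiles.
; BeginPlay starts the AIState's looping AIMoveTo behaviour, though Tick also calls ChasePlayer every frame without passing a target.
; Pawn sensing of BP_Player triggers a chase and launches impulse-driven projectiles.
; Hitbox overlaps damage players lacking invincibility frames, while bullets and explosions reduce Health with a material flicker until Tick destroys the actor.
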(event `self.ReceiveBeginPlay`
  ;[1 1 1] Makes My guy move, chase, and attack player
  (switch `/Game/Blueprints/Ivana_BP/EAIState` (`self.AIState`)
    (:`NewEnumerator1`
      (`self.Roam`))
    (:`NewEnumerator2`
      (`self.ChasePlayer` null))
    (:`NewEnumerator3`
      (`self.Patrol`))))

(event `Roam`
  ;[1 1 1] Makes My guy move, chase, and attack player
  (`|AIMoveTo` self (`NavigationSystemV1.K2_GetRandomLocationInNavigableRadius` (`self.K2_GetActorLocation`) 500.0 null null) null
    (:`OnSuccess`
      (`KismetSystemLibrary.Delay` 0.5)
      (`self.Roam`))))

(event `ChasePlayer`
  (params (PlayerToChase :type "Pawn Object Reference"))
  ;[1 1 1] Makes My guy move, chase, and attack player
  (`|AIMoveTo` self (0.0 0.0 0.0) PlayerToChase
    (:`OnSuccess`
      (`KismetSystemLibrary.Delay` 1.0)
      (`self.ChasePlayer` null))))

(event `Patrol`
  ;[1 1 1] Makes My guy move, chase, and attack player
  (`|AIMoveTo` self (0.0 0.0 0.0) (`self.TargetPoint1`)
    (:`OnSuccess`
      (`KismetSystemLibrary.Delay` 1.0)
      (`|AIMoveTo` self (0.0 0.0 0.0) (`self.TargetPoint2`)
        (:`OnSuccess`
          (`KismetSystemLibrary.Delay` 1.0)
          (`self.Patrol`))))))

(event `self.PawnSensing.OnSeePawn`
  (params (Pawn :type "Pawn Object Reference"))
  ;[1 1 1] Makes My guy move, chase, and attack player
  (bind _asbp_player (cast `/Game/Blueprints/ConnorBPs/Player/BP_Player` Pawn))
  (`|ExecutionSequence`
    (:`then_0`
      (`self.ChasePlayer` _asbp_player))
    (:`then_1`
      _))
  (if (`self.Spawn Projectile`)
    (bind _returnvalue (`|SpawnActorFromClass` "/Game/Blueprints/Ivana_BP/MyProjectile.MyProjectile_C" (`SceneComponent.K2_GetComponentToWorld` (`self.Projectile Spawn Location`)) "Undefined" "OverrideRootScale" null null))
    (`PrimitiveComponent.AddImpulse` (`/Game/Blueprints/Ivana_BP/MyProjectile.Sphere` _returnvalue) (* (`SceneComponent.GetForwardVector` (`self.RootComponent`)) (`self.ShootAmount`)) "None" true)
    (set `self.Spawn Projectile` true)
    (`KismetSystemLibrary.Delay` 0.25)
    (set `self.Spawn Projectile` true)))

(event `self.ReceiveTick`
  (params (DeltaSeconds :type "Float (single-precision)"))
  ;[1 1 1] activate chase on spawn and destroy actor when health is 0
  (`|ExecutionSequence`
    (:`then_0`
      (`self.chaseplayer` null))
    (:`then_1`
      (if (<= (`self.health`) 0)
        (`self.K2_DestroyActor`)))))

(event `self.Hitbox.OnComponentBeginOverlap`
  (params (OverlappedComponent :type "PrimitiveComponent Object Reference") (OtherActor :type "Actor Object Reference") (OtherComp :type "PrimitiveComponent Object Reference") (OtherBodyIndex :type Integer) (bFromSweep :type Boolean) (SweepResult :type "HitResult Structure (by ref)"))
  ;[1 1 1] when hit by bullet, decrement health
  (`|ExecutionSequence`
    (:`then_0`
      (cast `/Game/Blueprints/ConnorBPs/Projectiles/BP_Bullet` OtherActor)
      (`|ExecutionSequence`
        (:`then_0`
          (`/Engine/EditorBlueprintResources/StandardMacros.DecrementInt` (`self.health`)))
        (:`then_1`
          (`self.flicker`))))
    (:`then_1`
      (bind _asbp_player (cast `/Game/Blueprints/ConnorBPs/Player/BP_Player` OtherActor))
      (if (not (`/Game/Blueprints/ConnorBPs/Player/BP_Player.IFrame` _asbp_player))
        (set `/Game/Blueprints/ConnorBPs/Player/BP_Player.Player Health` (- (`/Game/Blueprints/ConnorBPs/Player/BP_Player.Player Health` _asbp_player) 0.1) _asbp_player)
        (`KismetSystemLibrary.PrintString` "Ouch!")
        (set `/Game/Blueprints/ConnorBPs/Player/BP_Player.IFrame` true _asbp_player)))
    (:`then_2`
      (cast `/Game/Blueprints/Colin_BPs/Explosion` OtherActor)
      (`|ExecutionSequence`
        (:`then_0`
          (for _ (range 5)
            (`/Engine/EditorBlueprintResources/StandardMacros.DecrementInt` (`self.health`))))
        (:`then_1`
          (`self.flicker`))))))

(event `flicker`
  (bind _mesh (`self.Mesh`))
  ;[1 1 1] Damage Indication
  (`PrimitiveComponent.SetMaterial` _mesh 0 "/Game/Blueprints/ConnorBPs/isOff.isOff")
  (`KismetSystemLibrary.Delay` 0.1)
  (`PrimitiveComponent.SetMaterial` _mesh 0 "/Game/Assets/Materials/Blue.Blue"))

(fn `GetRandomLocation`)

(fn `UserConstructionScript`)