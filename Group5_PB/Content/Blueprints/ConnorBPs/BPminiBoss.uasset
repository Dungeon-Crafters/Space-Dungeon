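; Mini-boss enemy that turns to face the player on sight and fires turret bullets on a cooldown.
; PawnSensing drives aiming and shooting, and can trigger a one-shot sound at the world origin.
; Hitbox overlaps with bullets or explosions reduce health and flicker the cube's material, while Tick destroys the actor at zero health.
; BeginPlay picks a random patrol point, but the timeline that would move between points is never triggered.
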(event `self.PawnSensing.OnSeePawn`
  (params (Pawn :type "Pawn Object Reference"))
  (if (`self.soundOn`)
    (`GameplayStatics.PlaySoundAtLocation` "/Game/StarterContent/Audio/Explosion01.Explosion01" (0.0 0.0 0.0) (struct) 1.0 1.0 0.0 null null null)
    (set `self.soundOn` false))
  (bind _asbp_player (cast `/Game/Blueprints/ConnorBPs/Player/BP_Player` Pawn))
  (`|ExecutionSequence`
    (:`then_0`
      (`self.K2_SetActorRotation` (`KismetMathLibrary.FindLookAtRotation` (`self.K2_GetActorLocation`) (`self.K2_GetActorLocation` _asbp_player))))
    (:`then_1`
      (if (`self.spawnprojectile`)
        (bind _returnvalue (`|SpawnActorFromClass` "/Game/Blueprints/Will_BPs/BP_TurretBullet.BP_TurretBullet_C" (`SceneComponent.K2_GetComponentToWorld` (`self.Scene`)) "Undefined" "OverrideRootScale" null null))
        (set `self.spawnprojectile` false)
        (`KismetSystemLibrary.Delay` 1.5)
        (set `self.spawnprojectile` true)))))

(event `self.ReceiveBeginPlay`
  (set `self.patrol points` (`|MakeArray` (`SceneComponent.K2_GetComponentLocation` (`self.Movepos1`)) (`SceneComponent.K2_GetComponentLocation` (`self.Movepos2`)) (`SceneComponent.K2_GetComponentLocation` (`self.Movepos3`))))
  (`self.GetRandomLocation`))

(event `flicker`
  (bind _cube (`self.Cube`))
  ;[1 1 1] Damage Indication
  (`PrimitiveComponent.SetMaterial` _cube 0 "/Game/Blueprints/ConnorBPs/isOff.isOff")
  (`KismetSystemLibrary.Delay` 0.1)
  (`PrimitiveComponent.SetMaterial` _cube 0 "/Game/Assets/Materials/Blue.Blue"))

(event `self.Hitbox.OnComponentBeginOverlap`
  (params (OverlappedComponent :type "PrimitiveComponent Object Reference") (OtherActor :type "Actor Object Reference") (OtherComp :type "PrimitiveComponent Object Reference") (OtherBodyIndex :type Integer) (bFromSweep :type Boolean) (SweepResult :type "HitResult Structure (by ref)"))
  (`|ExecutionSequence`
    (:`then_0`
      (cast `/Game/Blueprints/ConnorBPs/Projectiles/BP_Bullet` OtherActor)
      (`|ExecutionSequence`
        (:`then_0`
          (`/Engine/EditorBlueprintResources/StandardMacros.DecrementInt` (`self.health`)))
        (:`then_1`
          (`self.flicker`))))
    (:`then_1`
      (cast `/Game/Blueprints/Colin_BPs/Explosion` OtherActor)
      (`|ExecutionSequence`
        (:`then_0`
          (for _ (range 5)
            (`/Engine/EditorBlueprintResources/StandardMacros.DecrementInt` (`self.health`))))
        (:`then_1`
          (`self.flicker`))))))

(event `self.ReceiveTick`
  (params (DeltaSeconds :type "Float (single-precision)"))
  (if (<= (`self.health`) 0)
    (`self.K2_DestroyActor`)))

(fn `GetRandomLocation`
  (set `self.CurrentPatrolPoint` (`KismetMathLibrary.RandomInteger` (`KismetArrayLibrary.Array_Length` (`self.patrol points`)))))

(fn `UserConstructionScript`)