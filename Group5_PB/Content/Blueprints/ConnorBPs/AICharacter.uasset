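; Enemy AI character that chases the player after pawn sensing spots them and splits into smaller enemies on death.
; Chase re-issues AIMoveTo one second after each success; the first sighting also plays a beep.
; Hitbox overlaps apply bullet and explosion damage with a material flicker, or hurt the player outside invulnerability frames.
; Tick triggers SpawnMore at zero health, spawning AICharacterSmall pairs every frame until the delayed destroy.
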(event `self.PawnSensing.OnSeePawn`
  (params (Pawn :type "Pawn Object Reference"))
  ;[1 1 1] Switch from scout to alert
  (if (`self.soundOn`)
    (`GameplayStatics.PlaySoundAtLocation` "/Game/Assets/426888__thisusernameis__beep4.426888__thisusernameis__beep4" (0.0 0.0 0.0) (struct) 1.0 1.0 0.0 null null null)
    (set `self.soundOn` false))
  (cast `/Game/Blueprints/ConnorBPs/Player/BP_Player` Pawn)
  (`self.Chase`))

(event `Chase`
  ;[1 1 1] constant alert
  (`|AIMoveTo` self (0.0 0.0 0.0) (`GameplayStatics.GetPlayerPawn` 0)
    (:`OnSuccess`
      (`KismetSystemLibrary.Delay` 1.0)
      (`self.Chase`))))

(event `self.ReceiveTick`
  (params (DeltaSeconds :type "Float (single-precision)"))
  ;[1 1 1] Once health is 0, call death function
  (if (<= (`self.health`) 0)
    (`self.SpawnMore`)))

(event `self.Hitbox.OnComponentBeginOverlap`
  (params (OverlappedComponent :type "PrimitiveComponent Object Reference") (OtherActor :type "Actor Object Reference") (OtherComp :type "PrimitiveComponent Object Reference") (OtherBodyIndex :type Integer) (bFromSweep :type Boolean) (SweepResult :type "HitResult Structure (by ref)"))
  ;[1 1 1] When hit by bullet, decrease health
  (`|ExecutionSequence`
    (:`then_0`
      (cast `/Game/Blueprints/ConnorBPs/Projectiles/BP_Bullet` OtherActor)
      (`|ExecutionSequence`
        (:`then_0`
          (`/Engine/EditorBlueprintResources/StandardMacros.DecrementInt` (`self.health`)))
        (:`then_1`
          (`self.flicker`))))
    (:`then_1`
      (bind _asbp_player (cast `/Game/Blueprints/ConnorBPs/Player/BP_Player` OtherActor))
      (if (not (`/Game/Blueprints/ConnorBPs/Player/BP_Player.IFrame` _asbp_player))
        (set `/Game/Blueprints/ConnorBPs/Player/BP_Player.Player Health` (- (`/Game/Blueprints/ConnorBPs/Player/BP_Player.Player Health` _asbp_player) 0.1) _asbp_player)
        (`KismetSystemLibrary.PrintString` "Ouch!")
        (set `/Game/Blueprints/ConnorBPs/Player/BP_Player.IFrame` true _asbp_player)))
    (:`then_2`
      (cast `/Game/Blueprints/Colin_BPs/Explosion` OtherActor)
      (`|ExecutionSequence`
        (:`then_0`
          (for _ (range 5)
            (`/Engine/EditorBlueprintResources/StandardMacros.DecrementInt` (`self.health`))))
        (:`then_1`
          (`self.flicker`))))))

(event `flicker`
  (bind _cylinder (`self.Cylinder`))
  ;[1 1 1] Damage Indication
  (`PrimitiveComponent.SetMaterial` _cylinder 0 "/Game/Blueprints/ConnorBPs/isOff.isOff")
  (`KismetSystemLibrary.Delay` 0.1)
  (`PrimitiveComponent.SetMaterial` _cylinder 0 "/Game/Assets/Materials/Blue.Blue"))

(event `SpawnMore`
  (bind _returnvalue (`self.K2_GetActorLocation` self))
  ;[1 1 1] spawn a few enemies, kill parent object
  (`|ExecutionSequence`
    (:`then_0`
      (`AIBlueprintHelperLibrary.SpawnAIFromClass` "/Game/Blueprints/ConnorBPs/AICharacterSmall.AICharacterSmall_C" null _returnvalue))
    (:`then_1`
      (`AIBlueprintHelperLibrary.SpawnAIFromClass` "/Game/Blueprints/ConnorBPs/AICharacterSmall.AICharacterSmall_C" null _returnvalue))
    (:`then_2`
      (`KismetSystemLibrary.Delay` 0.2)
      (`self.K2_DestroyActor`))))

(fn `UserConstructionScript`)