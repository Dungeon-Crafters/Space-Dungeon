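; BP_Player is the playable character, handling movement, jumping, turning and grenade throwing.
; Input axes drive forward and strafe movement along actor vectors, while Aim offsets control yaw from actor yaw and zeroes pitch and roll.
; Right mouse spawns a scaled-down Grenade at the Sphere component with the camera's rotation, then launches it along camera forward by setting its physics velocity.
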(event `InputAction|Jump`
  (params (Key :type "Key Structure"))
  (:`Pressed`
    (`self.Jump`)))

(event `InputAxis|Move`
  (params (AxisValue :type "Float (single-precision)"))
  (`self.AddMovementInput` (`self.GetActorForwardVector`) AxisValue))

(event `InputAxis|Aim`
  (params (AxisValue :type "Float (single-precision)"))
  (bind (_returnvalue_roll _returnvalue_pitch _returnvalue_yaw) (`KismetMathLibrary.BreakRotator` (`self.K2_GetActorRotation`)))
  (`Controller.SetControlRotation` (`self.GetController`) (`KismetMathLibrary.MakeRotator` 0.0 0.0 (+ AxisValue _returnvalue_yaw))))

(event `InputAxis|Strafe`
  (params (AxisValue :type "Float (single-precision)"))
  (`self.AddMovementInput` (`self.GetActorRightVector`) AxisValue))

(event `Key|RightMouseButton`
  (params (Key :type "Key Structure"))
  (bind _returnvalue (`SceneComponent.K2_GetComponentRotation` (`self.Camera`)))
  ;[1 1 1] Throw Grenade
  (:`Pressed`
    (bind _returnvalue_2 (`|SpawnActorFromClass` "/Game/Blueprints/Colin_BPs/Grenade.Grenade_C" (`KismetMathLibrary.MakeTransform` (`SceneComponent.K2_GetComponentLocation` (`self.Sphere`)) _returnvalue (0.25 0.25 0.25)) "Undefined" "OverrideRootScale" null null))
    (`PrimitiveComponent.SetPhysicsLinearVelocity` (`/Game/Blueprints/Colin_BPs/Grenade.Sphere` _returnvalue_2) (* (`KismetMathLibrary.GetForwardVector` _returnvalue) 1500.0) false "None")))

(fn `UserConstructionScript`)