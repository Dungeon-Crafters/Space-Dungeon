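; GroundPoundBoss is an enemy that chases the player and destroys itself when its health runs out.
; Tick checks health and calls Assault every frame to issue AIMoveTo, which also re-calls itself after a delay on success.
; Hitbox overlaps take damage from bullets and explosions with a material flicker, or hurt the player unless IFrame is set.
; The Box overlap only prints a swing message; no ground-pound attack is implemented.
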(event `self.Box.OnComponentBeginOverlap`
  (params (OverlappedComponent :type "PrimitiveComponent Object Reference") (OtherActor :type "Actor Object Reference") (OtherComp :type "PrimitiveComponent Object Reference") (OtherBodyIndex :type Integer) (bFromSweep :type Boolean) (SweepResult :type "HitResult Structure (by ref)"))
  (cast `/Game/Blueprints/ConnorBPs/Player/BP_Player` OtherActor)
  (`KismetSystemLibrary.PrintString` "Enemy Swings at You")
  (`KismetSystemLibrary.Delay` 4.0))

(event `Assault`
  (`|AIMoveTo` self (0.0 0.0 0.0) (`GameplayStatics.GetPlayerPawn` 0)
    (:`OnSuccess`
      (`KismetSystemLibrary.Delay` 4.0)
      (`self.Assault`))))

(event `self.ReceiveTick`
  (params (DeltaSeconds :type "Float (single-precision)"))
  (`|ExecutionSequence`
    (:`then_0`
      (`self.Assault`))
    (:`then_1`
      (if (<= (`self.health`) 0)
        (`self.K2_DestroyActor`)))))

(event `flicker`
  (bind _mesh (`self.Mesh`))
  ;[1 1 1] Flicker
  (`PrimitiveComponent.SetMaterial` _mesh 0 "/Game/Blueprints/ConnorBPs/isOff.isOff")
  (`KismetSystemLibrary.Delay` 0.1)
  (`PrimitiveComponent.SetMaterial` _mesh 0 "/Game/Assets/Materials/Blue.Blue"))

(event `self.Hitbox.OnComponentBeginOverlap`
  (params (OverlappedComponent :type "PrimitiveComponent Object Reference") (OtherActor :type "Actor Object Reference") (OtherComp :type "PrimitiveComponent Object Reference") (OtherBodyIndex :type Integer) (bFromSweep :type Boolean) (SweepResult :type "HitResult Structure (by ref)"))
  ;[1 1 1] Health and flickering
  (`|ExecutionSequence`
    (:`then_0`
      (cast `/Game/Blueprints/ConnorBPs/Projectiles/BP_Bullet` OtherActor)
      (`|ExecutionSequence`
        (:`then_0`
          (`/Engine/EditorBlueprintResources/StandardMacros.DecrementInt` (`self.health`)))
        (:`then_1`
          (`self.flicker`))))
    (:`then_1`
      (bind _asbp_player (cast `/Game/Blueprints/ConnorBPs/Player/BP_Player` OtherActor))
      (if (not (`/Game/Blueprints/ConnorBPs/Player/BP_Player.IFrame` _asbp_player))
        (set `/Game/Blueprints/ConnorBPs/Player/BP_Player.Player Health` (- (`/Game/Blueprints/ConnorBPs/Player/BP_Player.Player Health` _asbp_player) 0.1) _asbp_player)
        (`KismetSystemLibrary.PrintString` "Ouch!")
        (set `/Game/Blueprints/ConnorBPs/Player/BP_Player.IFrame` true _asbp_player)))
    (:`then_2`
      (cast `/Game/Blueprints/Colin_BPs/Explosion` OtherActor)
      (`|ExecutionSequence`
        (:`then_0`
          (for _ (range 5)
            (`/Engine/EditorBlueprintResources/StandardMacros.DecrementInt` (`self.health`))))
        (:`then_1`
          (`self.flicker`))))))

(fn `UserConstructionScript`)