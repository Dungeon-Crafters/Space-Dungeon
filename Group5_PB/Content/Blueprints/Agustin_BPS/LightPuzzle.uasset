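; Light puzzle Blueprint that tracks how many lights count toward a win and moves a cube once all of them do.
; AddTo and RemoveFrom events raise and lower a counter, with the decrement clamped at zero.
; When the counter equals the number of Light actors in the level, WinCondition plays a timeline.
; The timeline adds its track value to the cube's relative Z location on every update.
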(event `AddTo`
  ;[1 1 1] Add untilInt is Equal to lights in the scene
  (set `self.int` (+ (`self.int`) 1))
  (bind _outactors (`GameplayStatics.GetAllActorsOfClass` "/Game/Blueprints/Agustin_BPS/Light.Light_C"))
  (if (== (`KismetArrayLibrary.Array_Length` _outactors) (`self.int`))
    (`self.WinCondition`)))

(event `WinCondition`
  (bind (_direction _newtrack_0) (`Timeline|WinnerWinner`)
    (:`Update`
      (`SceneComponent.K2_AddRelativeLocation` (`self.Cube`) (`KismetMathLibrary.MakeVector` 0.0 0.0 _newtrack_0) false false))))

(event `RemoveFrom`
  (bind _int (`self.int`))
  ;[1 1 1] TakeAway Int
  (if (> _int 0)
    (set `self.int` (- _int 1))))

(fn `UserConstructionScript`)