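; Enemy Blueprint that chases the player once PawnSensing spots them and explodes on reaching them.
; On first sighting it plays a beep, then uses AI Move To; success spawns an explosion emitter, destroys the enemy and reduces player health.
; Bullet overlaps on its hitbox lower its health and briefly flicker its materials.
; Tick destroys it without an explosion when health runs out.
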(event `self.PawnSensing.OnSeePawn`
  (params (Pawn :type "Pawn Object Reference"))
  (if (`self.soundOn`)
    (`GameplayStatics.PlaySoundAtLocation` "/Game/Assets/426888__thisusernameis__beep4.426888__thisusernameis__beep4" (0.0 0.0 0.0) (struct) 1.0 1.0 0.0 null null null)
    (set `self.soundOn` false))
  (bind _asbp_player (cast `/Game/Blueprints/ConnorBPs/Player/BP_Player` Pawn))
  (`|AIMoveTo` self (0.0 0.0 0.0) _asbp_player
    (:`OnSuccess`
      (`GameplayStatics.SpawnEmitterAtLocation` "/Game/StarterContent/Particles/P_Explosion.P_Explosion" (`self.K2_GetActorLocation`))
      (`self.K2_DestroyActor`)
      (bind _asbp_player_2 (cast `/Game/Blueprints/ConnorBPs/Player/BP_Player` _asbp_player))
      (set `/Game/Blueprints/ConnorBPs/Player/BP_Player.Player Health` (- (`/Game/Blueprints/ConnorBPs/Player/BP_Player.Player Health` _asbp_player_2) 0.3) _asbp_player_2)
      (`KismetSystemLibrary.PrintString` "Ouch!"))))

(event `flicker`
  (bind _enemy (`self.Enemy`))
  ;[1 1 1] Flicker
  (`PrimitiveComponent.SetMaterial` _enemy 0 "/Game/Blueprints/ConnorBPs/isOff.isOff")
  (`PrimitiveComponent.SetMaterial` (`self.Cone`) 0 "/Game/Blueprints/ConnorBPs/isOff.isOff")
  (`KismetSystemLibrary.Delay` 0.1)
  (`PrimitiveComponent.SetMaterial` _enemy 0 "/Game/Assets/Materials/Blue.Blue")
  (`PrimitiveComponent.SetMaterial` (`self.Cone`) 0 "/Game/Assets/Materials/Blue.Blue"))

(event `self.Hitbox.OnComponentBeginOverlap`
  (params (OverlappedComponent :type "PrimitiveComponent Object Reference") (OtherActor :type "Actor Object Reference") (OtherComp :type "PrimitiveComponent Object Reference") (OtherBodyIndex :type Integer) (bFromSweep :type Boolean) (SweepResult :type "HitResult Structure (by ref)"))
  ;[1 1 1] enemy health loss and I frames
  (cast `/Game/Blueprints/ConnorBPs/Projectiles/BP_Bullet` OtherActor)
  (`|ExecutionSequence`
    (:`then_0`
      (`/Engine/EditorBlueprintResources/StandardMacros.DecrementInt` (`self.Health`)))
    (:`then_1`
      (`self.flicker`))))

(event `self.ReceiveTick`
  (params (DeltaSeconds :type "Float (single-precision)"))
  ;[1 1 1] activate chase on spawn and destroy actor when health is 0
  (if (<= (`self.health`) 0)
    (`self.K2_DestroyActor`)))

(fn `UserConstructionScript`)