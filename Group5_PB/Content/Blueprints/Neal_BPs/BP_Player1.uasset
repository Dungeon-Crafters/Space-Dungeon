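; BP_Player1 is a player character that moves, strafes, jumps, turns by yaw only, fires bullets and throws grenades.
; Fire spawns BP_Bullet at a world-space offset along control rotation, while right mouse launches a physics grenade along the camera's forward vector.
; E toggles grabbing line-traced physics objects through a PhysicsHandle, whose target follows the HeldObject component every tick.
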(event `InputAction|Jump`
  (params (Key :type "Key Structure"))
  (:`Pressed`
    (`self.Jump`)))

(event `InputAxis|Move`
  (params (AxisValue :type "Float (single-precision)"))
  (`self.AddMovementInput` (`self.GetActorForwardVector`) AxisValue))

(event `InputAxis|Aim`
  (params (AxisValue :type "Float (single-precision)"))
  (bind (_returnvalue_roll _returnvalue_pitch _returnvalue_yaw) (`KismetMathLibrary.BreakRotator` (`self.K2_GetActorRotation`)))
  (`Controller.SetControlRotation` (`self.GetController`) (`KismetMathLibrary.MakeRotator` 0.0 0.0 (+ AxisValue _returnvalue_yaw))))

(event `InputAxis|Strafe`
  (params (AxisValue :type "Float (single-precision)"))
  (`self.AddMovementInput` (`self.GetActorRightVector`) AxisValue))

(event `Key|RightMouseButton`
  (params (Key :type "Key Structure"))
  (bind _returnvalue (`SceneComponent.K2_GetComponentRotation` (`self.Camera`)))
  ;[1 1 1] Throw Grenade
  (:`Pressed`
    (bind _returnvalue_2 (`|SpawnActorFromClass` "/Game/Blueprints/Colin_BPs/Grenade.Grenade_C" (`KismetMathLibrary.MakeTransform` (`SceneComponent.K2_GetComponentLocation` (`self.Sphere`)) _returnvalue (0.25 0.25 0.25)) "Undefined" "OverrideRootScale" null null))
    (`PrimitiveComponent.SetPhysicsLinearVelocity` (`/Game/Blueprints/Colin_BPs/Grenade.Sphere` _returnvalue_2) (* (`KismetMathLibrary.GetForwardVector` _returnvalue) 1500.0) false "None")))

(event `InputAction|Fire`
  (params (Key :type "Key Structure"))
  (bind _returnvalue_location (`KismetMathLibrary.BreakTransform` (`self.GetTransform`)))
  ;[1 1 1] Fire Bullet
  (:`Pressed`
    (`|SpawnActorFromClass` "/Game/Blueprints/ConnorBPs/Projectiles/BP_Bullet.BP_Bullet_C" (`KismetMathLibrary.MakeTransform` (+ (+ _returnvalue_location (0.0 -100.0 100.0)) (* (`self.GetActorRightVector`) 0.0)) (`self.GetControlRotation`) (0.25 0.25 0.25)) "Undefined" "OverrideRootScale" null null)))

(event `Key|E`
  (params (Key :type "Key Structure"))
  ;[1 1 1] Checks whether the player is holding an object when they press E
  (:`Pressed`
    (if (`self.Is_Holding_Object`)
      (`self.Drop Object`)
      (else
        (`self.Pickup Object`)))))

(event `Pickup Object`
  (bind _camera (`self.Camera`))
  (bind _returnvalue (`SceneComponent.K2_GetComponentLocation` _camera))
  ;[1 1 1] If the player was not holding an object, find an object in front of the player and pick it up
  (bind (_outhit _returnvalue_2) (`KismetSystemLibrary.LineTraceSingle` _returnvalue (+ (* (`SceneComponent.GetForwardVector` _camera) 10000.0) _returnvalue) "TraceTypeQuery1"))
  (if _returnvalue_2
    (`KismetSystemLibrary.PrintString` "Hit")
    (bind (_bblockinghit _binitialoverlap _time _distance _location _impactpoint _normal _impactnormal _physmat _hitactor _hitcomponent) (`GameplayStatics.BreakHitResult` _outhit))
    (if (`SceneComponent.IsSimulatingPhysics` _hitcomponent "None")
      (`PhysicsHandleComponent.GrabComponentAtLocation` (`self.PhysicsHandle`) _hitcomponent "None" (`SceneComponent.K2_GetComponentLocation` _hitcomponent))
      (set `self.Is_Holding_Object` true))
    (else
      (`KismetSystemLibrary.PrintString` "No Hit"))))

(event `Drop Object`
  ;[1 1 1] If holding an object when E is pressed, Drop it
  (`PhysicsHandleComponent.ReleaseComponent` (`self.PhysicsHandle`))
  (set `self.Is_Holding_Object` false))

(event `self.ReceiveTick`
  (params (DeltaSeconds :type "Float (single-precision)"))
  ;[1 1 1] Sets the picked up object to be in front of the player
  (`PhysicsHandleComponent.SetTargetLocation` (`self.PhysicsHandle`) (`SceneComponent.K2_GetComponentLocation` (`self.HeldObject`))))

(fn `UserConstructionScript`)